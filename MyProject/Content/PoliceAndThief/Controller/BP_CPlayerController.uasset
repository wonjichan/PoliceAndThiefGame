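; BP_CPlayerController is a player controller that shows a heart health HUD for the local player.
; On BeginPlay it casts the controlled pawn to BP_PlayerCharacter and binds to its HealthComponent's current HP change event.
; It then creates and adds WBP_HeartHUD to the viewport, refreshing the hearts whenever HP changes.
; Widget setup only happens on the local controller and only if the pawn cast succeeds.
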(event `self.ReceiveBeginPlay`
  (if (`self.IsLocalController`)
    (bind _asbp_player_character (cast `/Game/PoliceAndThief/Character/BP_PlayerCharacter` (`self.K2_GetPawn`)))
    (bind _output_get (set `self.PlayerCharacterRef` _asbp_player_character))
    (add `HealthComponent.OnCurrentHPChanged` (`PlayerCharacter.HealthComponent` _output_get) (delegate `OnHPChanged`))
    (bind _returnvalue (`|CreateWidget` "/Game/PoliceAndThief/UI/WBP_HeartHUD.WBP_HeartHUD_C"))
    (bind _output_get_2 (set `self.HeartWidget` _returnvalue))
    (`UserWidget.AddToViewport` _output_get_2 0)))

(event `OnHPChanged`
  (params (NewHP :type Integer))
  (`/Engine/EditorBlueprintResources/StandardMacros.IsValid` (`self.HeartWidget`)
    (:`Is Valid`
      (`/Game/PoliceAndThief/UI/WBP_HeartHUD.UpdateHeart` (`self.HeartWidget`)))))

(fn `UserConstructionScript`)